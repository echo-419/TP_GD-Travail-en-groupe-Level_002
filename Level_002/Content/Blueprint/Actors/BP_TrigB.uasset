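; BP_TrigB is a trigger actor that advances the Condition value stored on the GM_Main game mode.
; Any actor overlap reads Condition and raises it one step, from 0 up to 3, through a switch.
; The overlap does not filter the other actor, and the trigger stays active, so repeated overlaps keep advancing the value until it reaches 3.
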(event Collision|EventActorBeginOverlap
  (params (OtherActor :type Actor%20Object%20Reference))
  (bind _asgm_main (Utilities|Casting|CastToGM_Main (Game|GetGameMode)))
  (switch Utilities|FlowControl|Switch|SwitchonENUM_condition (Variables|/Game/Blueprint/Gamemodes/GM_Main.GM_Main_C|GetCondition _asgm_main)
    (:NewEnumerator0
      (bind _asgm_main_2 (Utilities|Casting|CastToGM_Main (Game|GetGameMode)))
      (Variables|/Game/Blueprint/Gamemodes/GM_Main.GM_Main_C|SetCondition _asgm_main_2 "NewEnumerator1"))
    (:NewEnumerator1
      (bind _asgm_main_3 (Utilities|Casting|CastToGM_Main (Game|GetGameMode)))
      (Variables|/Game/Blueprint/Gamemodes/GM_Main.GM_Main_C|SetCondition _asgm_main_3 "NewEnumerator2"))
    (:NewEnumerator2
      (bind _asgm_main_4 (Utilities|Casting|CastToGM_Main (Game|GetGameMode)))
      (Variables|/Game/Blueprint/Gamemodes/GM_Main.GM_Main_C|SetCondition _asgm_main_4 "NewEnumerator3"))))

(fn ConstructionScript)
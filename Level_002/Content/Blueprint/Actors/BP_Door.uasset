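; BP_Door is a door actor that opens once enough external conditions are met.
; OneMoreCondition increments a verified counter and opens the door when it equals the required count, while OneLessCondition decrements it and always closes the door.
; Opening plays a DoorOpening timeline that lerps the actor's yaw rotation; closing reverses it.
; The construction script resets the counter, and a GM_Main condition check is left unwired.
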(event Custom|OpenDoor
  ;[1 1 1] Animations
  (bind _doorrotation (Timeline|DoorOpening Play)
    (:Update
      (Transformation|SetActorRotation (Math|Rotator|Lerp(Rotator) "0, 0, 0" (Math|Rotator|MakeRotator 0.0 0.0 (Utilities|GETDOORZROT)) _doorrotation)))))

(event Custom|OneLessCondition
  ;[1 1 1] Conditions and INC/DECrementation
  (Math|Integer|DecrementInt (Variables|Default|GetM%20VerifiedCondition)
    (:%20%20
      (if true
        (CallFunction|CloseDoor)))))

(event Custom|CloseDoor
  ;[1 1 1] Animations
  (bind _doorrotation (Timeline|DoorOpening Reverse)
    (:Update
      (Transformation|SetActorRotation (Math|Rotator|Lerp(Rotator) "0, 0, 0" (Math|Rotator|MakeRotator 0.0 0.0 (Utilities|GETDOORZROT)) _doorrotation)))))

(event Custom|OneMoreCondition
  ;[1 1 1] Conditions and INC/DECrementation
  (bind _result (Math|Integer|IncrementInt (Variables|Default|GetM%20VerifiedCondition))
    (:%20%20
      (if (== (Variables|Default|GetM%20NbConditions) _result)
        (CallFunction|OpenDoor)))))

(fn ConstructionScript
  (Variables|Default|SetM%20VerifiedCondition 0))
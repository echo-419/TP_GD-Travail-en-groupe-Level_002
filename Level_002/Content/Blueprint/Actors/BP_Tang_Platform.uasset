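; Platform actor whose timeline is meant as a horizontal platform animation, started on BeginPlay only when MBeginFade is set.
; FadeIn plays PlatformAnimation and FadeOut reverses it, with the Finished event toggling MFade to pick the next direction and form a ping-pong loop.
; The timeline's ColorMultiplier feeds only an unreachable material-parameter call, so the graph applies no visible movement or fade.
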(event Custom|FadeIn
  ;[1 1 1] Horizontal Platform animation
  (bind _colormultiplier (Timeline|PlatformAnimation Play)
    (:Finished
      ;;[1 1 1] Resetting the operation
      (bind _output_get (Variables|Movement|SetM%20Fade (not (Variables|Movement|GetM%20Fade))))
      (if _output_get
        (CallFunction|FadeOut)
        (else
          (CallFunction|Fadein))))))

(event Custom|FadeOut
  ;[1 1 1] Horizontal Platform animation
  (bind _colormultiplier (Timeline|PlatformAnimation Reverse)
    (:Finished
      ;;[1 1 1] Resetting the operation
      (bind _output_get (Variables|Movement|SetM%20Fade (not (Variables|Movement|GetM%20Fade))))
      (if _output_get
        (CallFunction|FadeOut)
        (else
          (CallFunction|Fadein))))))

(event EventBeginPlay
  ;[1 1 1] Default call
  (if (Variables|Movement|GetM%20BeginFade)
    (CallFunction|Fadein)))

(fn ConstructionScript
  (Variables|Movement|SetM%20Fade true))
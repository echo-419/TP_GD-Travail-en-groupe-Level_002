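; Vertical moving platform actor that animates its mesh between its relative origin and a Z destination.
; If the begin-move flag is set, it starts on BeginPlay by playing a timeline whose ZForce track drives a lerp of the mesh's relative location, without sweeping.
; When the timeline finishes, it flips a direction flag and calls MoveUp or MoveDown to play or reverse it, keeping the motion cycling.
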(event Custom|MoveUp
  ;[1 1 1] Vertical Platform animation
  (bind _z_force (Timeline|PlatformAnimation Play)
    (:Update
      (Transformation|SetRelativeLocation (Variables|Default|GetPlatformMesh) (Math|Vector|Lerp(Vector) "0, 0, 0" (Math|Vector|MakeVector 0.0 0.0 (Variables|Ajust|GetM%20ZDestination)) _z_force) false false))
    (:Finished
      ;;[1 1 1] Resetting the direciton
      (bind _output_get (Variables|Movement|SetM%20MoveUp (not (Variables|Movement|GetM%20MoveUp))))
      (if _output_get
        (CallFunction|MoveDown)
        (else
          (CallFunction|MoveUp))))))

(event Custom|MoveDown
  ;[1 1 1] Vertical Platform animation
  (bind _z_force (Timeline|PlatformAnimation Reverse)
    (:Update
      (Transformation|SetRelativeLocation (Variables|Default|GetPlatformMesh) (Math|Vector|Lerp(Vector) "0, 0, 0" (Math|Vector|MakeVector 0.0 0.0 (Variables|Ajust|GetM%20ZDestination)) _z_force) false false))
    (:Finished
      ;;[1 1 1] Resetting the direciton
      (bind _output_get (Variables|Movement|SetM%20MoveUp (not (Variables|Movement|GetM%20MoveUp))))
      (if _output_get
        (CallFunction|MoveDown)
        (else
          (CallFunction|MoveUp))))))

(event EventBeginPlay
  ;[1 1 1] Default call
  (if (Variables|Movement|GetM%20BeginMove)
    (CallFunction|MoveUp)))

(fn ConstructionScript
  (Variables|Movement|SetM%20MoveUp true))
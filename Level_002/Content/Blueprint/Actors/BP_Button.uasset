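; BP_Button is a one-shot button actor that counts toward opening a linked door.
; On its BeingPressed event, the first press sets MPressed, calls OneMoreCondition on the referenced MDoor, and swaps the Sphere's material to Activated.
; Later presses are ignored; the construction script resets MPressed to false.
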(event Custom|BeingPressed
  (if (not (Variables|State|GetM%20Pressed))
    (Variables|State|SetM%20Pressed true)
    (Default|OneMoreCondition (Variables|Components|GetM%20Door))
    (Rendering|Material|SetMaterial (Variables|Default|GetSphere) 0 "/Game/Materials/Activated.Activated")))

(fn ConstructionScript
  (|CallParentFunction)
  (Variables|State|SetM%20Pressed false))
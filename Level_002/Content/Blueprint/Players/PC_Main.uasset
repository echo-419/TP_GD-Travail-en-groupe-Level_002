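; PC_Main is the player character Blueprint, handling movement, camera look, jumping, crouching and running from input events.
; Movement follows the camera's forward and right vectors, and look axes feed controller yaw and pitch.
; A counter reset on landing allows a double jump, crouch toggles, and holding run raises max walk speed.
; State variables initialise in the construction script; MCanInteract is never read, and the helper graphs are unfinished.
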(event EventOnLanded
  (params (Hit :type Hit%20Result%20Structure%20%28by%20ref%29))
  ;[1 1 1] saut
  (Variables|States|Setm_JumpCounter 0))

(event Input|ActionEvents|InputActionrun
  (params (Key :type Key%20Structure))
  (bind _charactermovement (Variables|Character|GetCharacterMovement))
  ;[1 1 1] run
  (:Pressed
    (Variables|/Script/Engine.CharacterMovementComponent|SetMaxWalkSpeed _charactermovement 1.5e+03))
  (:Released
    (Variables|/Script/Engine.CharacterMovementComponent|SetMaxWalkSpeed _charactermovement 5e+02)))

(event Input|ActionEvents|InputActionSaut
  (params (Key :type Key%20Structure))
  ;[1 1 1] saut
  (:Pressed
    (if (< (Variables|States|Getm_JumpCounter) 2)
      (Variables|States|Setm_PlayerState 0)
      (Math|Integer|IncrementInt (Variables|States|Getm_JumpCounter)
        (:%20%20
          (Character|Jump))))))

(event Input|ActionEvents|InputActioncrouch
  (params (Key :type Key%20Structure))
  ;[1 1 1] acroupit
  (:Pressed
    (if (AI|Components|NavMovement|IsCrouching (Variables|Character|GetCharacterMovement))
      (Character|UnCrouch)
      (else
        (Character|Crouch)))))

(event Input|AxisEvents|InputAxismoveStrafe
  (params (AxisValue :type Float%20%28single-precision%29))
  ;[1 1 1] déplacement
  (Pawn|Input|AddMovementInput (Math|Vector|GetRightVector (Variables|Default|GetCamera)) AxisValue false))

(event Input|AxisEvents|InputAxismoveForward
  (params (AxisValue :type Float%20%28single-precision%29))
  ;[1 1 1] déplacement
  (Pawn|Input|AddMovementInput (Math|Vector|GetForwardVector (Variables|Default|GetCamera)) AxisValue false))

(event Input|AxisEvents|InputAxislookX
  (params (AxisValue :type Float%20%28single-precision%29))
  ;[1 1 1] Camera
  (Pawn|Input|AddControllerYawInput AxisValue))

(event Input|AxisEvents|InputAxisLookY
  (params (AxisValue :type Float%20%28single-precision%29))
  ;[1 1 1] Camera
  (Pawn|Input|AddControllerPitchInput AxisValue))

(fn ConstructionScript
  (Variables|States|Setm_PlayerState 0)
  (Variables|States|Setm_JumpCounter 0)
  (Variables|States|Setm_CanInteract false))

(fn NewFunction0
  (params (self2 :type Character%20Movement%20Component%20Object%20Reference)))